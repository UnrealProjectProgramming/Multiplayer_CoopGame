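; Projectile Blueprint that explodes on a short fixed timer after BeginPlay, with no impact handling in its graphs.
; The Expload event spawns an explosion particle and applies radial damage at the actor's location, sized by DamageRadius and credited to its instigator controller.
; The actor is not destroyed afterward, and a debug sphere draw for the radius is left unconnected.
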(event `self.ReceiveBeginPlay`
  (`KismetSystemLibrary.Delay` 1.0)
  (`self.Expload`))

(event `Expload`
  (bind _returnvalue (`self.K2_GetActorLocation`))
  (`GameplayStatics.SpawnEmitterAtLocation` "/Game/WeaponEffects/Explosion/P_Explosion.P_Explosion" _returnvalue)
  (`GameplayStatics.ApplyRadialDamage` :`BaseDamage` 100.0 :`Origin` _returnvalue :`DamageRadius` (`self.DamageRadius`) :`DamageCauser` self :`InstigatedByController` (`self.GetInstigatorController`)))

(fn `UserConstructionScript`)