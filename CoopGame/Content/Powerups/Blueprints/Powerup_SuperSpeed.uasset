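; Super speed powerup that doubles the walk speed of the actor that activates it until the powerup expires.
; On activation it stores that actor and sets MaxWalkSpeed on its CharacterMovementComponent to twice the value of GetMaxSpeed.
; On expiry, if the actor is still valid, it halves the current max speed instead of restoring a saved value, then calls the parent expiry logic.
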(event `self.OnActivated`
  (params (ActivateForActor :type "Actor Object Reference"))
  (bind _returnvalue (`self.GetComponentByClass` ActivateForActor "/Script/Engine.CharacterMovementComponent"))
  (set `self.ActivatedForPlayers` ActivateForActor)
  (set `CharacterMovementComponent.MaxWalkSpeed` (* (`MovementComponent.GetMaxSpeed` _returnvalue) 2.0) _returnvalue))

(event `self.OnExpierd`
  (bind _activatedforplayers (`self.ActivatedForPlayers`))
  (bind _returnvalue (`self.GetComponentByClass` _activatedforplayers "/Script/Engine.CharacterMovementComponent"))
  (`/Engine/EditorBlueprintResources/StandardMacros.IsValid` _activatedforplayers
    (:`Is Valid`
      (set `CharacterMovementComponent.MaxWalkSpeed` (/ (`MovementComponent.GetMaxSpeed` _returnvalue) 2.0) _returnvalue))
    (:`Is Not Valid`
      _))
  (`parent.OnExpierd`))

(fn `UserConstructionScript`)