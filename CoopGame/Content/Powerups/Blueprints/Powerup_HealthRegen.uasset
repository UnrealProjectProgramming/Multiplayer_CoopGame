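; Health regeneration powerup that heals the local player over time while active.
; Powerup state changes toggle the HealthIcon, hiding it while the effect is active.
; Each powerup tick calls Heal with HealingAmount on the SHealthComponent of player pawn 0, regardless of who triggered it.
; The actor destroys itself when the powerup expires.
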(event `self.OnPowerStateChanged`
  (params (bNewIsActive :type Boolean))
  (`SceneComponent.SetVisibility` (`self.HealthIcon`) (not bNewIsActive) true))

(event `self.OnPowerupTicked`
  (bind _returnvalue (`self.GetComponentByClass` (`GameplayStatics.GetPlayerPawn` 0) "/Script/CoopGame.SHealthComponent"))
  (`/Engine/EditorBlueprintResources/StandardMacros.IsValid` _returnvalue
    (:`Is Valid`
      (`SHealthComponent.Heal` _returnvalue (`self.HealingAmount`)))))

(event `self.OnExpierd`
  (`self.K2_DestroyActor`))

(fn `UserConstructionScript`)